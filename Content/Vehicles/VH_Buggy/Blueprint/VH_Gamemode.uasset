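; Buggy game mode that runs the match countdown and ends the match by opening PostGameMap.
; BeginPlay loops on a one-second Delay, decrementing Seconds and Minutes, and repeats only while Seconds is nonzero.
; When both reach zero, it scans VH_BuggyP1 actors and stores any score beating WinningScore, with that player's name, in the GameManager game instance.
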(event `self.ReceiveBeginPlay`
  (`KismetSystemLibrary.Delay` 1.0 :!label _label)
  (set `self.seconds` (- (`self.seconds`) 1))
  (if (< (`self.seconds`) 0)
    (set `self.minutes` (- (`self.minutes`) 1))
    (set `self.seconds` 59))
  (if (== (`self.seconds`) 0)
    (if (== (`self.minutes`) 0)
      (bind _outactors (`GameplayStatics.GetAllActorsOfClass` "/Game/Vehicles/VH_Buggy/Blueprint/VH_BuggyP1.VH_BuggyP1_C"))
      (for _array_element _outactors
        (bind _asgame_manager (cast `/Game/Master/GameManager` (`GameplayStatics.GetGameInstance`)))
        (bind _playerscore (`/Game/Vehicles/VH_Buggy/Blueprint/VH_BuggyP1.PlayerScore` _array_element))
        (if (> _playerscore (`/Game/Master/GameManager.WinningScore` _asgame_manager))
          (set `/Game/Master/GameManager.WinningScore` _playerscore _asgame_manager)
          (set `/Game/Master/GameManager.WinningPlayer` (`/Game/Vehicles/VH_Buggy/Blueprint/VH_BuggyP1.PlayerName` _array_element) _asgame_manager)))
      (`GameplayStatics.OpenLevel` "PostGameMap"))
    (else
      (goto _label))))

(fn `UserConstructionScript`)