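; Weapon pickup actor that enables the first gun on a VH_Buggy that overlaps it.
; On overlap it sets Gun1Active, hides its skeletal mesh, then after a delay shows it again with an explosion effect and re-arms.
; A DoOnce gate ahead of the cast blocks repeat triggers, so a non-buggy overlap closes it with no reset.
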(event `self.ReceiveActorBeginOverlap`
  (params (OtherActor :type "Actor Object Reference"))
  (`/Engine/EditorBlueprintResources/StandardMacros.DoOnce` false :!label _label
    (:`Completed`
      (bind _asvh_buggy (cast `/Game/Vehicles/VH_Buggy/Blueprint/VH_Buggy` OtherActor))
      (set `/Game/Vehicles/VH_Buggy/Blueprint/VH_Buggy.Gun1Active?` true _asvh_buggy)
      (`SceneComponent.SetVisibility` (`self.SkeletalMesh`) false false)
      (`KismetSystemLibrary.Delay` 10.0)
      (`SceneComponent.SetVisibility` (`self.SkeletalMesh`) true false)
      (`GameplayStatics.SpawnEmitterAtLocation` "/Game/Effects/Effects/VehicleEffects/P_Explosion.P_Explosion" (`SceneComponent.K2_GetComponentLocation` (`self.SkeletalMesh`)))
      (goto _label :!via `Reset`))))

(fn `UserConstructionScript`)